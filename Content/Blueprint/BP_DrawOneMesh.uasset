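; Blueprint that builds one vertex-colored procedural mesh from vertex and triangle DataTables, then converts it to a named static mesh.
; DrawOneMesh calls GetData, which scales positions and shifts triangle indices to zero-based, then creates the section with a wall material.
; Each vertex's scalar Color value is normalized between Smallest and Biggest into a blue-green-red ramp.
; The range pre-pass skips zeros and only tests Smallest when a new Biggest is found.
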(event Custom|DrawOneMesh
  (bind _proceduralmesh (Variables|Default|GetProceduralMesh))
  (bind (_vertices _triangles _color) (CallFunction|GetData))
  (Class|ProceduralMeshComponent|CreateMeshSectionLinearColor _proceduralmesh 0 _vertices _triangles 0 0 0 0 0 _color 0 false)
  (Rendering|Material|SetMaterial _proceduralmesh 0 "/Game/StarterContent/Materials/M_Basic_Wall.M_Basic_Wall")
  (Class|PMConvertSM|ProceduralMeshConverttoStaticMesh (Variables|Default|GetProceduralMesh) (Variables|Default|GetMeshName))
  (Development|PrintString "Draw Over!"))

(fn ConstructionScript)

(fn GetData
  (bind _dt_vertices (Variables|Default|GetDT_Vertices))
  (CallFunction|CreateBiggestSmallest _dt_vertices)
  (bind _outrownames (DataTable|GetDataTableRowNames _dt_vertices))
  (for _array_element _outrownames
    (bind _returnvalue (Utilities|GetDataTableRow (Variables|Default|GetDT_Vertices) _array_element)
      (:then
        (Utilities|Array|Add (Variables|Default|GetVertices) (Math|Vector|MakeVector (* (.x (Utilities|Struct|Breakoutput_node_struct _returnvalue)) 2e+02) (* (.y (Utilities|Struct|Breakoutput_node_struct _returnvalue)) 2e+02) (* (.z (Utilities|Struct|Breakoutput_node_struct _returnvalue)) 2e+02)))
        (bind _newparam1 (CallFunction|ConverttoOne (.Color (Utilities|Struct|Breakoutput_node_struct _returnvalue))))
        (Utilities|Array|Add (Variables|Default|GetColor) _newparam1))))
  (bind _outrownames_2 (DataTable|GetDataTableRowNames (Variables|Default|GetDT_Triangles)))
  (for _array_element_2 _outrownames_2
    (bind _returnvalue_2 (Utilities|GetDataTableRow (Variables|Default|GetDT_Triangles) _array_element_2)
      (:then
        (Utilities|Array|Add (Variables|Default|GetTriangles) (- (.Vertice1 (Utilities|Struct|BreakS_Triangle _returnvalue_2)) 1))
        (Utilities|Array|Add (Variables|Default|GetTriangles) (- (.Vertice2 (Utilities|Struct|BreakS_Triangle _returnvalue_2)) 1))
        (Utilities|Array|Add (Variables|Default|GetTriangles) (- (.Vertice3 (Utilities|Struct|BreakS_Triangle _returnvalue_2)) 1)))))
  (return (Variables|Default|GetVertices) (Variables|Default|GetTriangles) (Variables|Default|GetColor)))

(fn ConverttoOne
  (params (NewParam :type Float%20%28single-precision%29))
  (bind _smallest (Variables|Default|GetSmallest))
  (bind _biggest (Variables|Default|GetBiggest))
  (bind _returnvalue (- NewParam _smallest))
  (bind _returnvalue_2 (- _biggest _smallest))
  (bind _returnvalue_3 (/ _returnvalue _returnvalue_2))
  (if (> _returnvalue_3 0.5)
    (Variables|Default|SetSingleColor (Utilities|Struct|MakeLinearColor (- (* _returnvalue_3 2.0) 1.0) (+ (* _returnvalue_3 -2.0) 2.0) 0.0 (+ _returnvalue_3 0.5)))
    (else
      (Variables|Default|SetSingleColor (Utilities|Struct|MakeLinearColor 0.0 (* _returnvalue_3 2.0) (+ (* _returnvalue_3 -2.0) 1.0) 1.0))))
  (return (Variables|Default|GetSingleColor)))

(fn CreateBiggestSmallest
  (params (NewParam :type Data%20Table%20Object%20Reference))
  (bind _outrownames (DataTable|GetDataTableRowNames NewParam))
  (for _array_element _outrownames
    (bind _returnvalue (Utilities|GetDataTableRow NewParam _array_element)
      (:then
        (if (not (== (.Color (Utilities|Struct|Breakoutput_node_struct _returnvalue)) 0.0))
          (if (> (.Color (Utilities|Struct|Breakoutput_node_struct _returnvalue)) (Variables|Default|GetBiggest))
            (Variables|Default|SetBiggest (.Color (Utilities|Struct|Breakoutput_node_struct _returnvalue)))
            (if (< (.Color (Utilities|Struct|Breakoutput_node_struct _returnvalue)) (Variables|Default|GetSmallest))
              (Variables|Default|SetSmallest (.Color (Utilities|Struct|Breakoutput_node_struct _returnvalue))))))))))