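; BP_myplane builds a color-coded 3D data visualization by spawning one BP_mymesh actor per data table row on BeginPlay.
; BigSmall first scans the table for the minimum and maximum Color values.
; Each row's X and Y set the mesh position, while its offset Color value times Z sets the vertical scale.
; Guiyihua normalizes that value into a blue-green-red gradient, applied through a dynamic material's Color parameter.
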(event EventBeginPlay
  (bind _datatable (Variables|Default|Getdatatable))
  ;[1 1 1] 根据点位生成Actor
  (CallFunction|BigSmall _datatable)
  (bind _outrownames (DataTable|GetDataTableRowNames _datatable))
  (for _array_element _outrownames
    (bind _returnvalue (Utilities|GetDataTableRow _datatable _array_element)
      (:then
        (bind _returnvalue_2 (Game|SpawnActorfromClass "/Game/Blueprint/BP_mymesh.BP_mymesh_C" (Math|Transform|MakeTransform (Math|Vector|MakeVector (* (.x (Utilities|Struct|Breakoutput_node_struct _returnvalue)) 1e+03) (* (.y (Utilities|Struct|Breakoutput_node_struct _returnvalue)) 1e+03) 0.0) "0, 0, 0" (Math|Vector|MakeVector 0.35 0.35 (* (- (.Color (Utilities|Struct|Breakoutput_node_struct _returnvalue)) 7e+01) (Variables|Default|Getz)))) "Undefined" 0 0))
        ;[1 1 1] 给每一个Actor的mesh创建一个动态材质
        (bind _returnvalue_3 (Rendering|Material|CreateDynamicMaterialInstance (Rendering|Material|GetMaterial (Variables|/Game/Blueprint/BP_mymesh.BP_mymesh_C|GetStaticMesh _returnvalue_2) 0) "None" :!class /Script/Engine.KismetMaterialLibrary))
        (Rendering|Material|SetMaterial (Variables|/Game/Blueprint/BP_mymesh.BP_mymesh_C|GetStaticMesh _returnvalue_2) 0 _returnvalue_3)
        (bind _newparam1 (CallFunction|Guiyihua (.Color (Utilities|Struct|Breakoutput_node_struct _returnvalue))))
        (Rendering|Material|SetVectorParameterValue _returnvalue_3 "Color" _newparam1 :!class /Script/Engine.MaterialInstanceDynamic)))))

(event Collision|EventActorBeginOverlap
  (params (OtherActor :type Actor%20Object%20Reference)))

(event EventTick
  (params (DeltaSeconds :type Float%20%28single-precision%29)))

(fn ConstructionScript)

(fn BigSmall
  (params (NewParam :type Data%20Table%20Object%20Reference))
  (bind _outrownames (DataTable|GetDataTableRowNames NewParam))
  (for _array_element _outrownames
    (bind _returnvalue (Utilities|GetDataTableRow NewParam _array_element)
      (:then
        (if (> (.Color (Utilities|Struct|Breakoutput_node_struct _returnvalue)) (Variables|Default|Getbiggest))
          (Variables|Default|Setbiggest (.Color (Utilities|Struct|Breakoutput_node_struct _returnvalue))))
        (if (< (.Color (Utilities|Struct|Breakoutput_node_struct _returnvalue)) (Variables|Default|Getsmallest))
          (Variables|Default|Setsmallest (.Color (Utilities|Struct|Breakoutput_node_struct _returnvalue))))))))

(fn Guiyihua
  (params (NewParam :type Float%20%28single-precision%29))
  (bind _smallest (Variables|Default|GetSmallest))
  (bind _biggest (Variables|Default|GetBiggest))
  (bind _returnvalue (- NewParam _smallest))
  (bind _returnvalue_2 (- _biggest _smallest))
  (bind _returnvalue_3 (/ _returnvalue _returnvalue_2))
  (if (> _returnvalue_3 0.5)
    (Variables|Default|SetNewVar_0 (Utilities|Struct|MakeLinearColor (- (* _returnvalue_3 2.0) 1.0) (+ (* _returnvalue_3 -2.0) 2.0) 0.0 1.0))
    (else
      (Variables|Default|SetNewVar_0 (Utilities|Struct|MakeLinearColor 0.0 (* _returnvalue_3 2.0) (+ (* _returnvalue_3 -2.0) 1.0) 1.0))))
  (return (Variables|Default|GetNewVar_0)))