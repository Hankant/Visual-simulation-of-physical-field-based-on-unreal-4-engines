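; Editor-style mesh builder that draws multiple meshes (stone blocks, per comments) from vertex and triangle DataTables and saves them as StaticMeshes.
; DrawMultipleMesh groups rows by consecutive MeshID into per-mesh arrays, converting triangle indices to zero-based.
; An ID change closes the current group without storing that row.
; Each group becomes a ProceduralMesh section, which a C++ function converts into a numbered StaticMesh asset.
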(event Custom|DrawMultipleMesh
  ;[1 0.1946 0.2364] 表格中的初始序号
  (Variables|Default|SetBeginNumber 1)
  ;[0.9586 1 0.4483] 将表格数据存放入数组中
  (bind _rowarray (CallFunction|InitReadData (Variables|Default|GetDT_Vertices)))
  (for _array_element _rowarray
    (Variables|Default|SetVerticeRow (Math|Conversions|ToInteger(Byte) (Utilities|String|ToString(Name) _array_element)))
    (bind _returnvalue (Class|DataTableFunctionLibrary|GetDataTableColumnasString (Variables|Default|GetDT_Vertices) "MeshID"))
    (bind _isequal (CallFunction|CompareNumber _returnvalue (Variables|Default|GetVerticeRow)))
    (if _isequal
      ;;[1 0.52 0.0299] 同一模型的顶点数据存入数组
      (CallFunction|SaveVerticeData)
      (else
        ;;[1 0.52 0.0299] 同一模型读入完毕，重置数组
        (CallFunction|AddVArrayandReset))))
  (bind _rowarray_2 (CallFunction|InitReadData (Variables|Default|GetDT_Triangles)))
  (for _array_element_2 _rowarray_2
    (Variables|Default|SetTriangleRow (Math|Conversions|ToInteger(Byte) (Utilities|String|ToString(Name) _array_element_2)))
    (bind _returnvalue_2 (Class|DataTableFunctionLibrary|GetDataTableColumnasString (Variables|Default|GetDT_Triangles) "MeshID"))
    (bind _isequal_2 (CallFunction|CompareNumber _returnvalue_2 (Variables|Default|GetTriangleRow)))
    (if _isequal_2
      ;;[1 0.52 0.0299] 同一模型的面片数据存入数组
      (CallFunction|SaveTriangleData)
      (else
        ;;[1 0.52 0.0299] 同一模型读入完毕，重置数组
        (CallFunction|AddTArrayandReset))))
  ;[0.6864 0.5905 1] 调用C++生成ProceduralMesh并转化为StaticMesh保存在Mesh文件夹下关闭前需要右键模型“资源本地化”->"重置化本地ID"
  (for _index (range (Variables|Default|GetBeginNumber) (- (Variables|Default|GetMeshNumber) 1))
    (Class|ProceduralMeshComponent|CreateMeshSectionLinearColor (Variables|组件|GetProceduralMesh) 0 (.permeshverticles (Utilities|Array|Get(acopy) (Variables|Default|Get2DVertices) _index)) (.permeshtriangles (Utilities|Array|Get(acopy) (Variables|Default|Get2DTriangles) _index)) 0 0 0 0 0 0 0 false)
    ;;[1 0.2833 0] PM转化SM算法
    (Class|PMConvertSM|ProceduralMeshConverttoStaticMesh (Variables|组件|GetProceduralMesh) (Utilities|String|Append (Variables|Default|GetMeshNamePrefix) (Utilities|String|ToString(Integer) _index))))
  (Development|PrintString "Draw Over!" true true "(R=0.362304,G=1.000000,B=0.000000,A=1.000000)" 4.0))

(fn ConstructionScript)

(fn SaveVerticeData
  ;[1 1 1] 同一石块的顶点数据存入数组
  (bind _returnvalue (Utilities|GetDataTableRow (Variables|Default|GetDT_Vertices) (Utilities|String|StringToName (Utilities|String|ToString(Integer) (Variables|Default|GetVerticeRow))))
    (:then
      (Utilities|Array|Add (Variables|Default|GetVerticesArray) (Math|Vector|MakeVector (.Vertice_X (Utilities|Struct|BreakS_Vertex _returnvalue)) (.Vertice_Y (Utilities|Struct|BreakS_Vertex _returnvalue)) (.Vertice_Z (Utilities|Struct|BreakS_Vertex _returnvalue)))))))

(fn AddVArrayandReset
  ;[1 1 1] 同一石块读入完毕，重置数组
  (Utilities|Array|SetArrayElem (Variables|Default|Get2DVertices) (Variables|Default|GetMeshNumber) (Utilities|Struct|MakeS_2DVertices (Variables|Default|GetVerticesArray)) true)
  (Variables|Default|SetMeshNumber (+ (Variables|Default|GetMeshNumber) 1))
  (Utilities|Array|Clear (Variables|Default|GetVerticesArray)))

(fn SaveTriangleData
  ;[1 1 1] 同一面片的面片数据存入数组
  (bind _returnvalue (Utilities|GetDataTableRow (Variables|Default|GetDT_Triangles) (Utilities|String|StringToName (Utilities|String|ToString(Integer) (Variables|Default|GetTriangleRow))))
    (:then
      (Utilities|Array|Add (Variables|Default|GetTrianglesArray) (- (.Vertice1 (Utilities|Struct|BreakS_Triangle _returnvalue)) 1))
      (Utilities|Array|Add (Variables|Default|GetTrianglesArray) (- (.Vertice2 (Utilities|Struct|BreakS_Triangle _returnvalue)) 1))
      (Utilities|Array|Add (Variables|Default|GetTrianglesArray) (- (.Vertice3 (Utilities|Struct|BreakS_Triangle _returnvalue)) 1)))))

(fn AddTArrayandReset
  ;[1 1 1] 同一石块读入完毕，重置数组
  (Utilities|Array|SetArrayElem (Variables|Default|Get2DTriangles) (Variables|Default|GetMeshNumber) (Utilities|Struct|MakeS_2DTriangles (Variables|Default|GetTrianglesArray)) true)
  (Variables|Default|SetMeshNumber (+ (Variables|Default|GetMeshNumber) 1))
  (Utilities|Array|Clear (Variables|Default|GetTrianglesArray)))

(fn CompareNumber
  (params (Array :type Array%20of%20Strings) (Row :type Integer))
  ;[1 1 1] 比较当前行的模型序号
  (bind _output_get (Variables|Default|SetCurrentNumber (Math|Conversions|ToInteger(Byte) (Utilities|Array|Get(acopy) Array (- Row (Variables|Default|GetBeginRow))))))
  (return (== _output_get (Variables|Default|GetMeshNumber))))

(fn InitReadData
  (params (DataTable :type Data%20Table%20Object%20Reference))
  ;[1 1 1] 赋变量初值
  (Variables|Default|SetMeshNumber (Variables|Default|GetBeginNumber))
  (bind _outrownames (DataTable|GetDataTableRowNames DataTable))
  (Variables|Default|SetBeginRow (Math|Conversions|ToInteger(Byte) (Utilities|String|ToString(Name) (Utilities|Array|Get(acopy) _outrownames))))
  (return _outrownames))