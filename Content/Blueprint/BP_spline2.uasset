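; Actor that draws data-table streamlines as splines and builds spline meshes colored by a scalar value.
; The construction script adds scaled row points, starting a new spline when the Streamline number changes, and collects Color values.
; BeginPlay finds the value range, then meshes only the last spline stored in Splinecontent.
; Each segment gets a dynamic material with its normalized value mapped to a blue-green-red gradient.
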(event EventBeginPlay
  (bind _splinecontent (Variables|Default|Getsplinecontent))
  (CallFunction|BigSmall false)
  (for _index (range 0 (- (Spline|GetNumberOfSplinePoints _splinecontent) 2))
    (bind _returnvalue (AddComponent|AddSplineMeshComponent true))
    (bind _returnvalue_2 (Rendering|Material|CreateDynamicMaterialInstance (Rendering|Material|GetMaterial _returnvalue 0) "None" :!class /Script/Engine.KismetMaterialLibrary))
    (Rendering|Material|SetMaterial _returnvalue 0 _returnvalue_2)
    (CallFunction|Guiyihua (Utilities|Array|Get(acopy) (Variables|Default|GetColors) _index))
    (Rendering|Material|SetVectorParameterValue _returnvalue_2 "Color" (Variables|Default|GetNewVar_4) :!class /Script/Engine.MaterialInstanceDynamic)
    (SplineMesh|SetStartandEnd _returnvalue (.Location (Spline|GetLocationandTangentatSplinePoint _splinecontent _index "World")) (.Tangent (Spline|GetLocationandTangentatSplinePoint _splinecontent _index "World")) (.Location (Spline|GetLocationandTangentatSplinePoint _splinecontent (+ _index 1) "World")) (.Tangent (Spline|GetLocationandTangentatSplinePoint _splinecontent (+ _index 1) "World")) true :!class /Script/Engine.SplineMeshComponent)))

(event Collision|EventActorBeginOverlap
  (params (OtherActor :type Actor%20Object%20Reference)))

(event EventTick
  (params (DeltaSeconds :type Float%20%28single-precision%29)))

(fn ConstructionScript
  (bind _spline_datatable (Variables|Default|Getspline_datatable))
  (bind _outrownames (DataTable|GetDataTableRowNames _spline_datatable))
  (for _array_element _outrownames
    (bind _returnvalue (Utilities|GetDataTableRow _spline_datatable _array_element)
      (:then
        (Utilities|Array|Add (Variables|Default|GetColors) (.Color (Utilities|Struct|BreakMyspline_struct _returnvalue)))
        (if (== (.Streamline (Utilities|Struct|BreakMyspline_struct _returnvalue)) (Variables|Default|Getlinenumber))
          (Class|SplineComponent|AddPoint (stale _returnvalue_2) (Utilities|Struct|MakeSplinePoint (Variables|Default|Getkey) (Math|Vector|MakeVector (* (.X (Utilities|Struct|BreakMyspline_struct _returnvalue)) 1e+03) (* (.Y (Utilities|Struct|BreakMyspline_struct _returnvalue)) 1e+03) (* (.Z (Utilities|Struct|BreakMyspline_struct _returnvalue)) 1e+03)) "0, 0,0.000000" "0, 0, 0" "0, 0, 0" "0, 0, 0" "Curve") true)
          (Variables|Default|Setkey (+ (Variables|Default|Getkey) 1.0))
          (Variables|Default|Setnumber (+ (Variables|Default|Getnumber) 1))
          (else
            (bind _returnvalue_2 (AddComponent|AddSplineComponent false))
            (Variables|Default|Setsplinecontent _returnvalue_2)
            (Spline|ClearSplinePoints _returnvalue_2 true)
            (Class|SplineComponent|AddPoint _returnvalue_2 (Utilities|Struct|MakeSplinePoint (Variables|Default|Getkey) (Math|Vector|MakeVector (* (.X (Utilities|Struct|BreakMyspline_struct _returnvalue)) 1e+03) (* (.Y (Utilities|Struct|BreakMyspline_struct _returnvalue)) 1e+03) (* (.Z (Utilities|Struct|BreakMyspline_struct _returnvalue)) 1e+03)) "0, 0, 0" "0, 0, 0" "0, 0, 0" "0, 0, 0" "Linear") true)
            (Variables|Default|Setlinenumber (+ (Variables|Default|Getlinenumber) 1.0))
            (Variables|Default|Setnumber (+ (Variables|Default|Getnumber) 1))))))))

(fn Guiyihua
  (params (NewParam :type Float%20%28single-precision%29))
  (bind _smallest (Variables|Default|GetSmallest))
  (bind _biggest (Variables|Default|GetBiggest))
  (bind _returnvalue (- NewParam _smallest))
  (bind _returnvalue_2 (- _biggest _smallest))
  (bind _returnvalue_3 (/ _returnvalue _returnvalue_2))
  (if (> _returnvalue_3 0.5)
    (Variables|Default|SetNewVar_4 (Utilities|Struct|MakeLinearColor (- (* _returnvalue_3 2.0) 1.0) (+ (* _returnvalue_3 -2.0) 2.0) 0.0 1.0))
    (else
      (Variables|Default|SetNewVar_4 (Utilities|Struct|MakeLinearColor 0.0 (* _returnvalue_3 2.0) (+ (* _returnvalue_3 -2.0) 1.0) 1.0)))))

(fn BigSmall
  (params (NewParam :type Boolean))
  (bind _spline_datatable (Variables|Default|Getspline_datatable))
  (bind _outrownames (DataTable|GetDataTableRowNames _spline_datatable))
  (for _array_element _outrownames
    (bind _returnvalue (Utilities|GetDataTableRow _spline_datatable _array_element)
      (:then
        (if (> (.Color (Utilities|Struct|BreakMyspline_struct _returnvalue)) (Variables|Default|Getbiggest))
          (Variables|Default|Setbiggest (.Color (Utilities|Struct|BreakMyspline_struct _returnvalue))))
        (if (< (.Color (Utilities|Struct|BreakMyspline_struct _returnvalue)) (Variables|Default|Getsmallest))
          (Variables|Default|Setsmallest (.Color (Utilities|Struct|BreakMyspline_struct _returnvalue))))))))