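; Actor that turns a static mesh into a procedural mesh and cuts it along a plane component when the slice event fires.
; The construction script copies the static mesh with collision, destroys the original and applies a brick material.
; Each slice caps the cut with a wall mask material, also applied to element 0, and makes the split-off half simulate physics with gravity.
; The plane then moves up 10 units.
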(event Custom|slice
  (bind _proceduralmesh (Variables|Default|GetProceduralMesh))
  (bind _plane (Variables|Default|GetPlane))
  (Rendering|Material|SetMaterial _proceduralmesh 0 "/Game/StarterContent/Materials/M_Basic_Wall_mask.M_Basic_Wall_mask")
  (bind _outotherhalfprocmesh (Class|KismetProceduralMeshLibrary|SliceProceduralMesh _proceduralmesh (Transformation|GetWorldLocation _plane) (Math|Vector|GetUpVector _plane) true "UseLastSectionForCap" "/Game/StarterContent/Materials/M_Basic_Wall_mask.M_Basic_Wall_mask"))
  (Physics|SetSimulatePhysics _outotherhalfprocmesh true)
  (Collision|SetCollisionEnabled _outotherhalfprocmesh "QueryAndPhysics")
  (Physics|SetEnableGravity _outotherhalfprocmesh true)
  (Transformation|AddRelativeLocation (Variables|Default|GetPlane) "0,0.000000,10.000000" false false))

(event EventBeginPlay)

(event Collision|EventActorBeginOverlap
  (params (OtherActor :type Actor%20Object%20Reference)))

(event EventTick
  (params (DeltaSeconds :type Float%20%28single-precision%29)))

(fn ConstructionScript
  (bind _proceduralmesh (Variables|Default|GetProceduralMesh))
  (bind _staticmesh (Variables|Default|GetStaticMesh))
  (Class|KismetProceduralMeshLibrary|CopyProceduralMeshfromStaticMeshComponent _staticmesh 0 _proceduralmesh true)
  (Components|DestroyComponent _staticmesh)
  (Rendering|Material|SetMaterial _proceduralmesh 0 "/Game/StarterContent/Materials/M_Brick_Clay_Old.M_Brick_Clay_Old"))