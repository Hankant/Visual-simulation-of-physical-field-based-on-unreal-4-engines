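; Blueprint that builds a procedural mesh from DataTables on DrawOneMesh and converts it to a named static mesh.
; GetData scans the vertex table's color range and reads triangle indices from the triangle table.
; Code filling vertex positions and colors, including the blue-green-red ConvertToOne gradient, is disconnected, so those arrays pass through unfilled.
; The minimum color updates only inside the new-maximum branch.
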(event Custom|DrawOneMesh
  (bind (_vertices _triangles _color) (CallFunction|GetData))
  (Class|ProceduralMeshComponent|CreateMeshSectionLinearColor (Variables|Default|GetProceduralMesh) 0 _vertices _triangles 0 0 0 0 0 _color 0 false)
  (Class|PMConvertSM|ProceduralMeshConverttoStaticMesh (Variables|Default|GetProceduralMesh) (Variables|Default|GetMeshName))
  (Development|PrintString "Draw Over!"))

(fn ConstructionScript)

(fn GetData
  (CallFunction|CreateBiggestSmallest (Variables|Default|GetDT_Vertices))
  (bind _outrownames (DataTable|GetDataTableRowNames (Variables|Default|GetDT_Triangles)))
  (for _array_element _outrownames
    (bind _returnvalue (Utilities|GetDataTableRow (Variables|Default|GetDT_Triangles) _array_element)
      (:then
        (Utilities|Array|Add (Variables|Default|GetTriangles) (.Vertice1 (Utilities|Struct|BreakS_Triangle _returnvalue)))
        (Utilities|Array|Add (Variables|Default|GetTriangles) (.Vertice2 (Utilities|Struct|BreakS_Triangle _returnvalue)))
        (Utilities|Array|Add (Variables|Default|GetTriangles) (.Vertice3 (Utilities|Struct|BreakS_Triangle _returnvalue))))))
  (return (Variables|Default|GetVertices) (Variables|Default|GetTriangles) (Variables|Default|GetColor)))

(fn ConverttoOne
  (params (NewParam :type Float%20%28single-precision%29))
  (bind _smallest (Variables|Default|GetSmallest))
  (bind _biggest (Variables|Default|GetBiggest))
  (bind _returnvalue (- NewParam _smallest))
  (bind _returnvalue_2 (- _biggest _smallest))
  (bind _returnvalue_3 (/ _returnvalue _returnvalue_2))
  (if (> _returnvalue_3 0.5)
    (Variables|Default|SetSingleColor (Utilities|Struct|MakeLinearColor (- (* _returnvalue_3 2.0) 1.0) (+ (* _returnvalue_3 -2.0) 2.0) 0.0 0.0))
    (else
      (Variables|Default|SetSingleColor (Utilities|Struct|MakeLinearColor 0.0 (* _returnvalue_3 2.0) (+ (* _returnvalue_3 -2.0) 1.0) 0.0))))
  (return (Variables|Default|GetSingleColor)))

(fn CreateBiggestSmallest
  (params (NewParam :type Data%20Table%20Object%20Reference))
  (bind _outrownames (DataTable|GetDataTableRowNames NewParam))
  (for _array_element _outrownames
    (bind _returnvalue (Utilities|GetDataTableRow NewParam _array_element)
      (:then
        (if (> (.Color (Utilities|Struct|Breakoutput_node_struct _returnvalue)) (Variables|Default|GetBiggest))
          (Variables|Default|SetBiggest (.Color (Utilities|Struct|Breakoutput_node_struct _returnvalue)))
          (if (< (.Color (Utilities|Struct|Breakoutput_node_struct _returnvalue)) (Variables|Default|GetSmallest))
            (Variables|Default|SetSmallest (.Color (Utilities|Struct|Breakoutput_node_struct _returnvalue)))))))))